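; BP_MainCharacterController is the main character's controller, creating the WB_UI widget on BeginPlay and acting as the bridge between gameplay and that UI.
; The I key flip-flops between the inventory screen and the HUD.
; Custom events forward hunger and health stats, add or refresh inventory entries, and open the inventory in its alternate mode filled with a shop's items.
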(event EventBeginPlay
  (bind _returnvalue (UserInterface|CreateWidget "/Game/AppointmentContents/UI/Widgets/WB_UI.WB_UI_C" (Game|GetPlayerController 0) 0))
  (Variables|Default|SetWB_UI _returnvalue)
  (UserInterface|Viewport|AddtoViewport _returnvalue 0))

(event EventTick
  (params (DeltaSeconds :type Float%20%28single-precision%29)))

(event EventUpdateStats
  (params (NewHunger :type Float%20%28single-precision%29) (NewHealth :type Float%20%28single-precision%29))
  (Default|UpdateStats (Variables|Default|GetWB_UI) NewHunger NewHealth))

(event EventOpenShop
  (params (OwningShop :type Shop%20Keeper%20Object%20Reference) (Items :type Array%20of%20Item%20Data%20Structures))
  (bind _wb_ui (Variables|Default|GetWB_UI))
  (Default|Inventory _wb_ui true)
  (Default|AddShopItems (Variables|/Game/AppointmentContents/UI/Widgets/WB_UI.WB_UI_C|GetWB_Inventory _wb_ui) Items OwningShop))

(event EventAddItemandUpdateInventoryWidget
  (params (ItemData :type Item%20Data%20Structure) (CurrentInventory :type Array%20of%20Item%20Data%20Structures))
  (bind _wb_ui (Variables|Default|GetWB_UI))
  (bind _wb_inventory (Variables|/Game/AppointmentContents/UI/Widgets/WB_UI.WB_UI_C|GetWB_Inventory _wb_ui))
  (bind _addnewitem (Default|ShouldAddNewItem _wb_inventory CurrentInventory true))
  (if _addnewitem
    (Default|AddItem _wb_inventory true ItemData)
    (else
      (Default|Update _wb_inventory true CurrentInventory))))

(event Input|KeyboardEvents|I
  (params (Key :type Key%20Structure :default "None"))
  (bind _wb_ui (Variables|Default|GetWB_UI))
  (:Pressed
    (Utilities|FlowControl|FlipFlop
      (:A
        (Default|Inventory _wb_ui false))
      (:B
        (Default|HUD _wb_ui)))))

(fn ConstructionScript)